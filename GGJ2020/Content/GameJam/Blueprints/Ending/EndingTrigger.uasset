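; EndingTrigger is a trigger actor that starts the game's ending when a BP_Golem enters its volume.
; After a short delay, CommenceEnding spawns an EMP with sound at the Golem's location, destroys every Launcher and plays an explosion sound.
; It then shows the WBP_Ending widget and switches to UI-only input with a visible cursor.
; An alternative path that polls all Golems for overlap is left unconnected.
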(event OnComponentBeginOverlap(Trigger)
  (params (OverlappedComponent :type Primitive%20Component%20Object%20Reference) (OtherActor :type Actor%20Object%20Reference) (OtherComp :type Primitive%20Component%20Object%20Reference) (OtherBodyIndex :type Integer) (bFromSweep :type Boolean) (SweepResult :type Hit%20Result%20Structure%20%28by%20ref%29))
  (bind _asbp_golem (Utilities|Casting|CastToBP_Golem OtherActor))
  (Utilities|FlowControl|Delay 1.5)
  (CallFunction|CommenceEnding (Transformation|GetActorLocation _asbp_golem)))

(fn ConstructionScript)

(fn CommenceEnding
  (params (Location :type Vector))
  (bind _returnvalue (Game|GetPlayerController 0))
  (bind _returnvalue_2 (Game|SpawnActorfromClass "/Game/GameJam/Blueprints/Ending/EMP.EMP_C" (Math|Transform|MakeTransform Location "0, 0, 0" "1,1,1") "AlwaysSpawn" 0 0))
  (Variables|Default|SetEMP _returnvalue_2)
  ;[1 1 1] Sound einfügen
  (Audio|PlaySoundatLocation "/Game/GameJam/Audio/SFX/Cue_EMP.Cue_EMP" Location "0, 0, 0" 1.0 1.0 0.0 0 0 0)
  (bind _outactors (Actor|GetAllActorsOfClass "/Game/GameJam/Blueprints/AI/Launcher.Launcher_C"))
  (for _array_element _outactors
    (Actor|DestroyActor _array_element))
  (Audio|PlaySound2D "/Game/GameJam/Audio/SFX/Cue_Explosion.Cue_Explosion" 1.0 1.0 0.0 0 0)
  (bind _returnvalue_3 (UserInterface|CreateWidget "/Game/GameJam/Blueprints/Widgets/WBP_Ending.WBP_Ending_C"))
  (UserInterface|Viewport|AddtoViewport _returnvalue_3 5)
  (Input|SetInputModeUIOnly _returnvalue 0 "DoNotLock")
  (Variables|/Script/Engine.PlayerController|SetbShowMouseCursor _returnvalue true))